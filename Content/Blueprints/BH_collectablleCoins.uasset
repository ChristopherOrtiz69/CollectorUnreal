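; Collectable coin actor that spins in place and adds to the third-person character's coin count on overlap.
; Tick yaws the Mesh by RotationSpeed each frame, without delta-time scaling.
; PickUpRadius overlap casts the other actor's Instigator to BP_ThirdPersonCharacter, increments its Coins and prints the result.
; The coin is not destroyed or hidden after pickup.
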(event `self.ReceiveTick`
  (params (DeltaSeconds :type "Float (single-precision)"))
  (`SceneComponent.K2_AddRelativeRotation` (`self.Mesh`) (`KismetMathLibrary.MakeRotator` 0.0 0.0 (`self.RotationSpeed`)) false false))

(event `self.PickUp Radius.OnComponentBeginOverlap`
  (params (OverlappedComponent :type "PrimitiveComponent Object Reference") (OtherActor :type "Actor Object Reference") (OtherComp :type "PrimitiveComponent Object Reference") (OtherBodyIndex :type Integer) (bFromSweep :type Boolean) (SweepResult :type "HitResult Structure (by ref)"))
  (bind _asbp_third_person_character (cast `/Game/Blueprints/BP_ThirdPersonCharacter` (`self.GetInstigator` OtherActor)))
  (bind _result (`/Engine/EditorBlueprintResources/StandardMacros.IncrementInt` (`/Game/Blueprints/BP_ThirdPersonCharacter.Coins` _asbp_third_person_character))
    (:`  `
      (`KismetSystemLibrary.PrintString` (`KismetStringLibrary.Conv_IntToString` _result)))))

(fn `UserConstructionScript`)